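; BP_MiniGrassBlock is a mini grass block actor that moves up and down continuously from BeginPlay.
; A Timeline track sets its world Z each update while keeping X and Y.
; On finish, the IsUp flag flips to choose between reversing and playing from the start, looping the motion.
; A Box physics-velocity check is left unconnected.
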(event EventBeginPlay
  (bind _returnvalue (Transformation|GetActorLocation))
  (bind _newtrack_0 (Timeline|Timeline Play)
    (:Update
      (Transformation|SetActorLocation (Math|Vector|MakeVector (.x _returnvalue) (.y _returnvalue) _newtrack_0) false false))
    (:Finished
      (bind _output_get (Variables|Default|SetIsUp (not (Variables|Default|GetIsUp))))
      (if _output_get
        (Timeline|Timeline Reverse)
        (else
          (Timeline|Timeline PlayFromStart))))))

(event Collision|EventActorBeginOverlap
  (params (OtherActor :type Actor%20Object%20Reference)))

(event EventTick
  (params (DeltaSeconds :type Float%20%28single-precision%29)))

(fn ConstructionScript)
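; BP_MiniBlock is a mini block actor that registers itself with the player's BP_MinecraftSteve character on overlap.
; BeginPlay caches player 0's character, and an overlap by any Steve sets that cached character's Item to this block.
; An unconnected Timeline would ping-pong the block's world Z to bob it up and down, but it never runs, nor does a debug name print.
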(event EventBeginPlay
  (bind _asbp_minecraft_steve (Utilities|Casting|CastToBP_MinecraftSteve (Game|GetPlayerCharacter 0)))
  (Variables|Default|SetPlayerCharacter _asbp_minecraft_steve))

(event Collision|EventActorBeginOverlap
  (params (OtherActor :type Actor%20Object%20Reference))
  (Utilities|Casting|CastToBP_MinecraftSteve OtherActor)
  (Variables|/Game/Blueprints/BP_MinecraftSteve.BP_MinecraftSteve_C|SetItem (Variables|Default|GetPlayerCharacter) self))

(fn ConstructionScript)
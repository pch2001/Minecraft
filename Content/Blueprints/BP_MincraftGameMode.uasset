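; Game mode for a Minecraft-style world that sets up terrain noise and spawns the starting chunks.
; On BeginPlay it constructs a FastNoiseWrapper configured for Perlin noise and stores it as SurfaceNoise.
; It then spawns a two-by-two grid of BP_WorldManager actors at fixed spacing, giving each its ChunckCoordinates.
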(event EventBeginPlay
  (Utilities|FlowControl|Sequence
    (:then_0
      (bind _returnvalue (Game|ConstructObjectfromClass "/Script/FastNoiseGenerator.FastNoiseWrapper"))
      (bind _output_get (Variables|Default|SetSurfaceNoise _returnvalue))
      (Class|FastNoiseWrapper|SetupFastNoise _output_get "Perlin" 1337 0.02 "Quintic" "FBM" 3 2.0 0.5 0.45 "Euclidean" "CellValue"))
    (:then_1
      (for _index (range 0 1)
        (for _index_2 (range 0 1)
          (Game|SpawnActorfromClass "/Game/Blueprints/Block/ISM/BP_WorldManager.BP_WorldManager_C" (Math|Transform|MakeTransform (* (Math|Vector|MakeVector (Math|Conversions|ToFloat(Integer) _index) (Math|Conversions|ToFloat(Integer) _index_2) 0.0) 1600) "0, 0, 0" "1.000000,1.000000,1.000000") "Undefined" "MultiplyWithRoot" 0 (Math|Vector|MakeVector (Math|Conversions|ToFloat(Integer) _index) (Math|Conversions|ToFloat(Integer) _index_2) 0.0) 0))))))

(event EventTick
  (params (DeltaSeconds :type Float%20%28single-precision%29)))

(fn ConstructionScript)
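; Grid component that converts a position into a location snapped to a grid of GridSize cells.
; GetGridLocation rounds each axis of Location to the nearest GridSize multiple, then adds NormalLocation scaled by GridSize to offset along that direction.
; Event graph stubs are disabled, and leftover debug and BP_WorldManager hit-lookup nodes never run.
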(event EventBeginPlay)

(event EventTick
  (params (DeltaSeconds :type Float%20%28single-precision%29)))

(fn GetGridLocation
  (params (Location :type Vector) (NormalLocation :type Vector))
  (bind _gridsize (Variables|Default|GetGridSize))
  (bind _gridsize_2 (Variables|Default|GetGridSize))
  (return (+ (* NormalLocation _gridsize) (Math|Vector|MakeVector (* (Math|Conversions|ToFloat(Integer) (Math|Float|Round (/ (.x Location) _gridsize))) _gridsize_2) (* (Math|Conversions|ToFloat(Integer) (Math|Float|Round (/ (.y Location) _gridsize))) _gridsize_2) (* (Math|Conversions|ToFloat(Integer) (Math|Float|Round (/ (.z Location) _gridsize))) _gridsize_2)))))
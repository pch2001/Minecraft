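; BP_Block is a mineable block actor that shows breaking progress and drops an item when broken.
; InItBlock copies its row from DT_BlockCSV into DefaultData and clears the crack progress on the cube.
; AddMineProgress drives the "BrokeFininsh" material parameter from progress over break time, then spawns the drop and destroys the block at 80%.
; ResetProgress clears that parameter; the stored effective tool is not checked here.
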(event Custom|AddMineProgress
  (params (CurrentProgress :type Float%20%28double-precision%29))
  (bind _defaultdata (Variables|Default|GetDefaultData))
  (bind _returnvalue (/ CurrentProgress (.broketime _defaultdata)))
  (Rendering|Material|SetScalarParameterValueonMaterials (Variables|Default|GetCube) "BrokeFininsh" _returnvalue)
  (if (>= _returnvalue 0.8)
    (Game|SpawnActorfromClass (.dropitem (Variables|Default|GetDefaultData)) (Transformation|GetWorldTransform (Variables|Default|GetDefaultSceneRoot)) "Undefined" "MultiplyWithRoot" 0 0)
    (Actor|DestroyActor)))

(event Custom|ResetProgress
  (Rendering|Material|SetScalarParameterValueonMaterials (Variables|Default|GetCube) "BrokeFininsh" 0.0))

(event Custom|InItBlock
  (params (Row_Name :type Name))
  (bind _returnvalue (Utilities|GetDataTableRow "/Game/Blueprints/Block/BlockData/DT_BlockCSV.DT_BlockCSV" Row_Name)
    (:then
      (Variables|Default|SetDefaultData (Utilities|Struct|MakeS_BlocksData (.Number (Utilities|Struct|BreakS_BlocksData _returnvalue)) (.ID (Utilities|Struct|BreakS_BlocksData _returnvalue)) (.Texture (Utilities|Struct|BreakS_BlocksData _returnvalue)) (.BrokeTime (Utilities|Struct|BreakS_BlocksData _returnvalue)) (.DropItem (Utilities|Struct|BreakS_BlocksData _returnvalue)) (.EffectiveTool (Utilities|Struct|BreakS_BlocksData _returnvalue)) 0 0))
      (Rendering|Material|SetScalarParameterValueonMaterials (Variables|Default|GetCube) "BrokeFininsh" 0.0))))

(event EventBeginPlay)

(fn ConstructionScript)
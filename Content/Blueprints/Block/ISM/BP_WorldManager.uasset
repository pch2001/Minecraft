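; Minecraft-style world manager that builds a chunk of instanced blocks and handles their mining and placement.
; On BeginPlay it creates one ISM component per DT_BlockCSV row, then stacks surface and underground blocks offset by the game mode's 2D noise.
; Damage events write mining progress to per-instance custom data.
; At 80% progress it spawns the drop item, hides the instance by zero-scaling it and resets the player's mine timer.
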(event Custom|DamageBlock
  (params (Time :type Float%20%28double-precision%29) (ItemNumber :type Integer) (Index_Item :type Integer))
  (bind _worldblockdataarray (Variables|Default|GetWorldBlockDataArray))
  (bind _output (Utilities|Array|Get(acopy) _worldblockdataarray ItemNumber))
  (bind (_number _id _texture _broketime) (Utilities|Struct|BreakS_BlocksData _output))
  (bind _returnvalue (/ Time _broketime))
  (bind _result (Math|Integer|IncrementInt Index_Item)
    (:%20%20
      (Variables|Default|SetTempItemNumber ItemNumber)
      (bind _returnvalue_2 (Components|InstancedStaticMesh|SetCustomDataValue (.Value (Utilities|Map|GetKeyValueByIndex (Variables|Default|GetISM_Map) _result)) (Variables|Default|GetTempItemNumber) 1 _returnvalue true))
      (if _returnvalue_2
        (if (>= _returnvalue 0.8)
          (bind _returnvalue_3 (Utilities|GetDataTableRow "/Game/Blueprints/Block/BlockData/DT_BlockCSV.DT_BlockCSV" (.Key (Utilities|Map|GetKeyValueByIndex (Variables|Default|GetISM_Map) _result)))
            (:then
              (Game|SpawnActorfromClass (Utilities|Struct|BreakS_BlocksData _returnvalue_3) (Math|Transform|MakeTransform (.location (.OutInstanceTransform (Components|InstancedStaticMesh|GetInstanceTransform (.Value (Utilities|Map|GetKeyValueByIndex (Variables|Default|GetISM_Map) _result)) (Variables|Default|GetTempItemNumber) true))) (.rotation (.OutInstanceTransform (Components|InstancedStaticMesh|GetInstanceTransform (.Value (Utilities|Map|GetKeyValueByIndex (Variables|Default|GetISM_Map) _result)) (Variables|Default|GetTempItemNumber) true))) "1.000000,1.000000,1.000000") "Undefined" "MultiplyWithRoot" 0 0)
              (Components|InstancedStaticMesh|UpdateInstanceTransform (.Value (Utilities|Map|GetKeyValueByIndex (Variables|Default|GetISM_Map) _result)) (Variables|Default|GetTempItemNumber) (Math|Transform|MakeTransform "0, 0, 0" "0, 0, 0" "0.000000,0.000000,0.000000") false false false)
              (bind _asbp_minecraft_steve (Utilities|Casting|CastToBP_MinecraftSteve (Game|GetPlayerCharacter 0)))
              (Default|ResetMineTime _asbp_minecraft_steve))))
        (else
          (Development|PrintString "NoCustomDataValue"))))))

(event Custom|ResetDamage
  (params (ItemNumber :type Integer) (TargetComponentNumber :type Integer))
  (bind _returnvalue (+ TargetComponentNumber 1))
  (bind _ism_map (Variables|Default|GetISM_Map))
  (bind (_key _value) (Utilities|Map|GetKeyValueByIndex _ism_map _returnvalue))
  (Components|InstancedStaticMesh|SetCustomDataValue _value ItemNumber 1 0.0 true)
  (Development|PrintString "Reset")
  (Development|PrintString (Utilities|String|ToString(Name) _key)))

(event Custom|IntancedStaticMeshSpawn
  (params (Instance%20Transform%20Location :type Vector) (TargetComponentNumber :type Integer))
  (bind _returnvalue (Components|InstancedStaticMesh|AddInstance (.Value (Utilities|Map|GetKeyValueByIndex (Variables|Default|GetISM_Map) TargetComponentNumber)) (Math|Transform|MakeTransform Instance%20Transform%20Location "0, 0, 0" "1.000000,1.000000,1.000000") true)))

(event Custom|SearchLocation
  (params (Item%20Index :type Integer) (TargetComponentNumber :type Integer))
  (Development|PrintString (Utilities|String|ToString(Vector) (.location (.OutInstanceTransform (Components|InstancedStaticMesh|GetInstanceTransform (.Value (Utilities|Map|GetKeyValueByIndex (Variables|Default|GetISM_Map) (+ TargetComponentNumber 1))) Item%20Index true))))))

(event EventBeginPlay
  (bind _ism_map (Variables|Default|GetISM_Map))
  (bind _ism_map_2 (Variables|Default|GetISM_Map))
  (bind _targetblockname (Variables|Default|GetTargetBlockName))
  (bind _targetblockname2 (Variables|Default|GetTargetBlockName2))
  (bind (_value _returnvalue) (Utilities|Map|Find _ism_map _targetblockname2))
  (bind (_value_2 _returnvalue_2) (Utilities|Map|Find _ism_map_2 _targetblockname))
  (Utilities|FlowControl|Sequence
    (:then_0
      (bind _asbp_mincraft_game_mode (Utilities|Casting|CastToBP_MincraftGameMode (Game|GetGameMode)))
      (Variables|Default|SetAs%20BP%20Mincraft%20Game%20Mode _asbp_mincraft_game_mode)
      (Development|PrintString "success"))
    (:then_1
      ;[0.15 0.15 0.15 0.5] 블럭 로드
      (bind _outrownames (DataTable|GetDataTableRowNames "/Game/Blueprints/Block/BlockData/DT_BlockCSV.DT_BlockCSV"))
      (for _array_element _outrownames
        (bind _returnvalue_3 (Utilities|GetDataTableRow "/Game/Blueprints/Block/BlockData/DT_BlockCSV.DT_BlockCSV" _array_element)
          (:then
            (bind _returnvalue_4 (AddComponent|AddInstancedStaticMeshComponent false (Math|Transform|MakeTransform "1.000000,1.000000,1.000000" "0, 0, 0" "1.000000,1.000000,1.000000")))
            (Components|StaticMesh|SetStaticMesh _returnvalue_4 "/Game/Blueprints/Block/Cube.Cube")
            (Rendering|Material|SetMaterial _returnvalue_4 0 (.BlockMaterias (Utilities|Struct|BreakS_BlocksData _returnvalue_3)))
            (Collision|SetCollisionObjectType _returnvalue_4 "ECC_WorldStatic")
            ;;[0.15 0.15 0.15 0.5] Comment
            (Class|InstancedStaticMeshComponent|SetNumCustomDataFloats _returnvalue_4 100)
            (Utilities|Map|Add (Variables|Default|GetISM_Map) _array_element _returnvalue_4))))
      (Utilities|FlowControl|Delay 0.1)
      (for _index (range 0 (Variables|Default|GetSpawnSize)) ; z
        (for _index_2 (range 0 (Variables|Default|GetSpawnSize)) ; y
          (for _index_3 (range 0 (Variables|Default|GetSpawnSize)) ; x
            (if (!= _index 0)
              (if _returnvalue
                (Components|InstancedStaticMesh|AddInstance _value (Math|Conversions|ToTransform(Vector) (+ (* (Math|Vector|MakeVector (Math|Conversions|ToFloat(Integer) _index_3) (Math|Conversions|ToFloat(Integer) _index_2) (Math|Conversions|ToFloat(Integer) _index)) "100.000000,100.000000,-100.000000") (Math|Vector|MakeVector 0.0 0.0 (Math|Float|SnapToGrid(Float) (* (Class|FastNoiseWrapper|GetNoise2D (Variables|/Game/Blueprints/BP_MincraftGameMode.BP_MincraftGameMode_C|GetSurfaceNoise (Variables|Default|GetAs%20BP%20Mincraft%20Game%20Mode)) (.x (+ (Math|Vector|MakeVector (Math|Conversions|ToFloat(Integer) _index_3) (Math|Conversions|ToFloat(Integer) _index_2) 0.0) (* (Variables|Default|GetChunckCoordinates) (Variables|Default|GetSpawnSize)))) (.y (+ (Math|Vector|MakeVector (Math|Conversions|ToFloat(Integer) _index_3) (Math|Conversions|ToFloat(Integer) _index_2) 0.0) (* (Variables|Default|GetChunckCoordinates) (Variables|Default|GetSpawnSize))))) 1e+03) 1e+02)))) false)
                (bind _returnvalue_5 (Utilities|GetDataTableRow "/Game/Blueprints/Block/BlockData/DT_BlockCSV.DT_BlockCSV" (Variables|Default|GetTargetBlockName2))
                  (:then
                    (Utilities|Array|Add (Variables|Default|GetWorldBlockDataArray) _returnvalue_5)))
                (else
                  (Development|PrintString "No Search" true true "(R=0.000000,G=0.660000,B=1.000000,A=1.000000)" 1e+01 :!label _label)))
              (elif _returnvalue_2
                (Components|InstancedStaticMesh|AddInstance _value_2 (Math|Conversions|ToTransform(Vector) (+ (* (Math|Vector|MakeVector (Math|Conversions|ToFloat(Integer) _index_3) (Math|Conversions|ToFloat(Integer) _index_2) (Math|Conversions|ToFloat(Integer) _index)) "100.000000,100.000000,-100.000000") (Math|Vector|MakeVector 0.0 0.0 (Math|Float|SnapToGrid(Float) (* (Class|FastNoiseWrapper|GetNoise2D (Variables|/Game/Blueprints/BP_MincraftGameMode.BP_MincraftGameMode_C|GetSurfaceNoise (Variables|Default|GetAs%20BP%20Mincraft%20Game%20Mode)) (.x (+ (Math|Vector|MakeVector (Math|Conversions|ToFloat(Integer) _index_3) (Math|Conversions|ToFloat(Integer) _index_2) 0.0) (* (Variables|Default|GetChunckCoordinates) (Variables|Default|GetSpawnSize)))) (.y (+ (Math|Vector|MakeVector (Math|Conversions|ToFloat(Integer) _index_3) (Math|Conversions|ToFloat(Integer) _index_2) 0.0) (* (Variables|Default|GetChunckCoordinates) (Variables|Default|GetSpawnSize))))) 1e+03) 1e+02)))) false)
                (bind _returnvalue_6 (Utilities|GetDataTableRow "/Game/Blueprints/Block/BlockData/DT_BlockCSV.DT_BlockCSV" (Variables|Default|GetTargetBlockName))
                  (:then
                    (Utilities|Array|Add (Variables|Default|GetWorldBlockDataArray) _returnvalue_6)))
                (else
                  (goto _label))))))))))

(fn ConstructionScript)
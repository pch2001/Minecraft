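; BP_MapSpawner generates a solid volume of BP_GrassBlock actors when play begins.
; Three nested loops on BeginPlay walk fixed X, Y and Z index ranges, spawning one block per cell at the index vector scaled by GridSize.
; The horizontal ranges start away from zero, so the volume is offset from the world origin rather than placed relative to the spawner.
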(event EventBeginPlay
  (for _index (range 10 20)
    (for _index_2 (range 10 20)
      (for _index_3 (range 0 10)
        (Game|SpawnActorfromClass "/Game/Blueprints/Block/BP_GrassBlock.BP_GrassBlock_C" (Math|Conversions|ToTransform(Vector) (* (Math|Vector|MakeVector (Math|Conversions|ToFloat(Integer) _index) (Math|Conversions|ToFloat(Integer) _index_2) (Math|Conversions|ToFloat(Integer) _index_3)) (Variables|Default|GetGridSize))) "Undefined" "MultiplyWithRoot" 0 0)))))

(fn ConstructionScript)
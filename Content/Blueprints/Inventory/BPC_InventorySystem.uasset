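; Inventory component that stores items in a fixed-size array of slots, sized to InventorySize at BeginPlay.
; AddItem places items one unit at a time, topping up a matching stack below its DT_Item StackSize, otherwise filling the first empty slot, and stops when none remains.
; ChangeSlot swaps slots within or between inventory components, only when their item names differ; same-item stacks are not merged.
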(event EventBeginPlay
  (Utilities|Array|Resize (Variables|Default|GetSlots) (Variables|Default|GetInventorySize)))

(event EventTick
  (params (DeltaSeconds :type Float%20%28single-precision%29)))

(fn AddItem
  (params (ItemAmount :type Integer) (ItemKey :type Name))
  (LocalVariables|SetAmountLeft ItemAmount)
  (LocalVariables|SetLocalItemKey ItemKey)
  (while (and (> (LocalVariables|GetAmountLeft) 0) (not (Variables|Default|GetIsAddFailed)))
    (bind (_arrayindexs _foundslot) (CallFunction|FindSlot (LocalVariables|GetLocalItemKey))) ; 인벤토리에서 찾는다
    (if _foundslot ; 인벤토리에서 똑같은걸 찾았다면?
      (CallFunction|IncreaseSlotStack _arrayindexs 1)
      (Math|Integer|DecrementInt (LocalVariables|GetAmountLeft)
        (:%20%20
          (Development|PrintString "Fine Same")))
      (elif (.IsSlotAvailable (CallFunction|CheckSlotEmpty)) ; 인벤토리에서 찾지 못했다면
        (CallFunction|AddtoNewSlot (LocalVariables|GetLocalItemKey) 1) ; 새로운 슬롯 추가
        (Math|Integer|DecrementInt (LocalVariables|GetAmountLeft))
        (else
          (Variables|Default|SetIsAddFailed true))))))

(fn FindSlot
  (params (ItemKey :type Name))
  (LocalVariables|SetTempItemKey ItemKey)
  (for (_array_element _array_index) (Variables|Default|GetSlots)
    (if (== (.Item_Name (Utilities|Struct|BreakS_Slot _array_element)) (LocalVariables|GetTempItemKey)) ; 인벤토리의 슬롯에 있는 아이템의 ItemName\n이 방금주운 아이템과 같다면
      (if (< (.Amount (Utilities|Struct|BreakS_Slot _array_element)) (CallFunction|GetStackSize (LocalVariables|GetTempItemKey))) ; 아이템의 최대stackSize가\n인벤토리에 있는 아이템의 개수보다 적다면?
        (Development|PrintString (Utilities|String|ToString(Text) (Utilities|Text|FormatText "item : {one} find {two}" (LocalVariables|GetTempItemKey) (Utilities|String|ToString(Integer) _array_index))))
        (return _array_index true))))
  (return -1 false))

(fn GetStackSize
  (params (ItemKey :type Name))
  (bind _returnvalue (Utilities|GetDataTableRow "/Game/Blueprints/MiniBlock/DT_Item.DT_Item" ItemKey)
    (:then
      (return (.StackSize (Utilities|Struct|BreakS_Item _returnvalue))))
    (:RowNotFound
      (return -1))))

(fn IncreaseSlotStack
  (params (Index :type Integer) (Amount :type Integer))
  (bind _slots (Variables|Default|GetSlots))
  (bind _output (Utilities|Array|Get(acopy) _slots Index))
  (bind (_item_name _amount) (Utilities|Struct|BreakS_Slot _output))
  (Utilities|Array|SetArrayElem (Variables|Default|GetSlots) Index (Utilities|Struct|MakeS_Slot _item_name (+ Amount _amount))))

(fn CheckSlotEmpty
  (for (_array_element _array_index) (Variables|Default|GetSlots)
    (if (== (.Amount (Utilities|Struct|BreakS_Slot _array_element)) 0) ; 슬록의 아이템 개수가 0
      (return true _array_index)))
  (return false -1) ; 인벤토리를 전부 돌 아봤는데 \n수가 0인 슬롯이 없다면 -1
)

(fn AddtoNewSlot
  (params (ItemKey :type Name) (Amount :type Integer))
  (Utilities|Array|SetArrayElem (Variables|Default|GetSlots) (.EmptyslotIndex (CallFunction|CheckSlotEmpty)) (Utilities|Struct|MakeS_Slot ItemKey Amount)))

(fn ChangeSlot
  (params (TargetIndex :type Integer) (BeforeInventory :type BPC%20Inventory%20System%20Object%20Reference) (Beforeindex :type Integer))
  (LocalVariables|SetLocalSlot (Utilities|Array|Get(acopy) (Variables|BPC_InventorySystem_C|GetSlots BeforeInventory) Beforeindex))
  (if (>= TargetIndex 0)
    (if (!= (.Item_Name (Utilities|Struct|BreakS_Slot (LocalVariables|GetLocalSlot))) (.Item_Name (Utilities|Struct|BreakS_Slot (Utilities|Array|Get(acopy) (Variables|Default|GetSlots) TargetIndex))))
      (Utilities|Array|SetArrayElem (Variables|BPC_InventorySystem_C|GetSlots BeforeInventory) Beforeindex (Utilities|Array|Get(acopy) (Variables|Default|GetSlots) TargetIndex))
      (Utilities|Array|SetArrayElem (Variables|Default|GetSlots) TargetIndex (LocalVariables|GetLocalSlot)))))